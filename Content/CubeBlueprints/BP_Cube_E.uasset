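; BP_Cube_E is an actor that randomly changes its static mesh material when another actor begins overlapping it.
; A chain of three branches picks one of three material variables and applies it to element 0.
; Each branch makes a fresh random roll, so the odds favor MaterialOne and some overlaps leave the material unchanged.
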(event Collision|EventActorBeginOverlap
  (params (OtherActor :type Actor%20Object%20Reference))
  (bind _returnvalue (Math|Random|RandomInteger 3))
  (bind _staticmeshcomponent (Variables|Debug|GetStaticMeshComponent))
  (if (== _returnvalue 0)
    (Rendering|Material|SetMaterial _staticmeshcomponent 0 "/Game/CubeBlueprints/MaterialOne.MaterialOne")
    (elif (== _returnvalue 1)
      (Rendering|Material|SetMaterial _staticmeshcomponent 0 "/Game/CubeBlueprints/MaterialTwo.MaterialTwo")
      (elif (== _returnvalue 2)
        (Rendering|Material|SetMaterial _staticmeshcomponent 0 "/Game/CubeBlueprints/MaterialThree.MaterialThree")))))

(fn ConstructionScript)