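; BP_Cube_F is a moving guard cube that sends characters back to a fixed location on contact.
; On BeginPlay, the GuardBox timeline drives the static mesh along Y while holding X and Z constant.
; Overlapping a BP_Cube_A stops the timeline, freezing the guard.
; Any other overlapping Character has its root component set to a hardcoded position without sweep or teleport, despite the "Kill" label.
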(event Custom|Forwards
  ;[1 1 1] Movement
  (bind _newtrack_0 (Timeline|guardBox Play)
    (:Update
      (Transformation|SetRelativeLocation (Variables|Debug|GetStaticMeshComponent) (Math|Vector|MakeVector 8e+02 (.y _newtrack_0) 3.5e+02) false false))))

(event Custom|Stop
  ;[1 1 1] Movement
  (bind _newtrack_0 (Timeline|guardBox Stop)
    (:Update
      (Transformation|SetRelativeLocation (Variables|Debug|GetStaticMeshComponent) (Math|Vector|MakeVector 8e+02 (.y _newtrack_0) 3.5e+02) false false))))

(event Collision|EventActorBeginOverlap
  (params (OtherActor :type Actor%20Object%20Reference))
  ;[1 1 1] Stop & Kill Player
  (Utilities|Casting|CastToBP_Cube_A OtherActor
    (:then
      (CallFunction|Stop))
    (:CastFailed
      (bind _ascharacter (Utilities|Casting|CastToCharacter OtherActor))
      (Transformation|SetRelativeLocation (Variables|/Script/Engine.Actor|GetRootComponent _ascharacter) "-499.999985,600.000063,392.000000" false false))))

(event EventBeginPlay
  ;[1 1 1] Movement
  (CallFunction|Forwards))

(fn ConstructionScript)