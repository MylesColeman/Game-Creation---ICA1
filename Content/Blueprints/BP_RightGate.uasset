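; BP_RightGate is a gate actor that swings open once the player has the key and sets the next objective.
; An external Transform event marks the key as held; a later overlap plays a ding and a one-shot timeline.
; The timeline drives the actor's yaw and, on each update, sets the player character's current objective to entering the warehouse.
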(event EventBeginPlay
  (bind _asbp_character (Utilities|Casting|CastToBP_Character (Game|GetPlayerCharacter 0))))

(event EventTransform
  (Variables|Default|SethasKey true))

(event Collision|EventActorBeginOverlap
  (params (OtherActor :type Actor%20Object%20Reference))
  (if (Variables|Default|GethasKey)
    (Utilities|FlowControl|DoOnce false
      (:Completed
        (Audio|PlaySound2D "/Game/Assets/Interaction_Ding.Interaction_Ding" 1.0 1.0 0.0 0 0)
        (bind _gate_open (Timeline|Gate Play)
          (:Update
            (Transformation|SetActorRotation (Math|Rotator|MakeRotator 0.0 0.0 (.z _gate_open)))
            (Variables|/Game/Characters/BP_Character.BP_Character_C|SetcurrentObj (stale EventBeginPlay _asbp_character) "Enter the warehouse")))))))

(fn ConstructionScript)