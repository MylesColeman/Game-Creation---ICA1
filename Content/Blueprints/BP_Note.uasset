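; BP_Note is an interactable note that grants the player a password on first interaction.
; A DoOnce gate makes Interact fire once, playing a ding and setting HasPassword.
; It disables the cached BP_Character's input and raises its NoteInteract flag for a few seconds, then restores both.
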(event EventBeginPlay
  (bind _asbp_character (Utilities|Casting|CastToBP_Character (Game|GetPlayerCharacter 0))))

(event EventInteract
  (Utilities|FlowControl|DoOnce false
    (:Completed
      (Audio|PlaySound2D "/Game/Assets/Interaction_Ding.Interaction_Ding" 1.0 1.0 0.0 0 0)
      (Variables|Default|SethasPassword true)
      (Input|DisableInput (stale EventBeginPlay _asbp_character) 0)
      (Variables|/Game/Characters/BP_Character.BP_Character_C|SetnoteInteract (stale EventBeginPlay _asbp_character) true)
      (Utilities|FlowControl|Delay 3.0)
      (Variables|/Game/Characters/BP_Character.BP_Character_C|SetnoteInteract (stale EventBeginPlay _asbp_character) false)
      (Input|EnableInput (stale EventBeginPlay _asbp_character) 0))))

(fn ConstructionScript)