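; BP_Spike is a hazard that damages the player while something overlaps it.
; BeginPlay caches the player character as BP_Character, and overlap begin and end events toggle an Overlapping flag for any actor.
; Tick runs through a one-second Delay, so it applies fixed damage about once per second while the flag is set, always to the cached player rather than the overlapping actor.
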(event Collision|EventActorBeginOverlap
  (params (OtherActor :type Actor%20Object%20Reference))
  (Variables|Default|Setoverlapping true))

(event Collision|EventActorEndOverlap
  (params (OtherActor :type Actor%20Object%20Reference))
  (Variables|Default|Setoverlapping false))

(event EventTick
  (params (DeltaSeconds :type Float%20%28single-precision%29))
  (Utilities|FlowControl|Delay 1.0)
  (if (Variables|Default|Getoverlapping)
    (Game|Damage|ApplyDamage (stale EventBeginPlay _output_get) 1e+01 0 0)))

(event EventBeginPlay
  (bind _asbp_character (Utilities|Casting|CastToBP_Character (Game|GetPlayerCharacter 0)))
  (bind _output_get (Variables|Default|SetAs%20BP%20Character _asbp_character)))

(fn ConstructionScript)